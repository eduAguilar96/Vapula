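; Base projectile Blueprint that delivers a damage payload to whatever its Bullet component hits.
; SetDamageInfo stores the damage range, crit chance and elemental amounts on the projectile.
; On hit, it spawns impact effects, passes that payload with bone name and instigator to actors implementing DamageInterface, then destroys itself.
; An actor overlap sets a short lifespan instead of dealing damage.
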(event OnComponentHit(Bullet)
  (params (HitComponent :type Primitive%20Component%20Object%20Reference) (OtherActor :type Actor%20Object%20Reference) (OtherComp :type Primitive%20Component%20Object%20Reference) (NormalImpulse :type Vector :default "0, 0, 0") (Hit :type Hit%20Result%20Structure%20%28by%20ref%29))
  (bind (_bblockinghit _binitialoverlap _time _location _impactpoint _normal _impactnormal _physmat _hitactor _hitcomponent _hitbonename) (Collision|BreakHitResult Hit))
  (Effects|SpawnEmitteratLocation (Variables|Default|GetImpactEffect) _impactpoint)
  (Audio|PlaySoundatLocation 0 _impactpoint)
  (if (Utilities|DoesObjectImplementInterface _hitactor "/Game/Interfaces/DamageInterface.DamageInterface_C")
    (Class|DamageInterface|TakeDamage(Message) _hitactor (Variables|Default|GetDamageMin) (Variables|Default|GetDamageMax) (Variables|Default|GetDamageCritChance) (Variables|Default|GetDamageFire) (Variables|Default|GetDamageElectric) (Variables|Default|GetDamageCorrosive) (Variables|Default|GetDamageIceWater) (Variables|Default|GetDamageExplosive) _hitbonename (Game|GetInstigator)))
  (Actor|DestroyActor))

(event EventBeginPlay)

(event Collision|EventActorBeginOverlap
  (params (OtherActor :type Actor%20Object%20Reference))
  (Actor|SetLifeSpan 3.0))

(event EventTick
  (params (DeltaSeconds :type Float%20%28single-precision%29)))

(fn ConstructionScript)

(fn SetDamageInfo
  (params (DamageMin :type Float%20%28single-precision%29) (DamageMax :type Float%20%28single-precision%29) (DamageCritChance :type Float%20%28single-precision%29) (DamageFire :type Float%20%28single-precision%29) (DamageElectric :type Float%20%28single-precision%29) (DamageCorrosive :type Float%20%28single-precision%29) (DamageIceWater :type Float%20%28single-precision%29) (DamageExplosive :type Float%20%28single-precision%29))
  (Variables|Default|SetDamageMin DamageMin)
  (Variables|Default|SetDamageMax DamageMax)
  (Variables|Default|SetDamageCritChance DamageCritChance)
  (Variables|Default|SetDamageFire DamageFire)
  (Variables|Default|SetDamageElectric DamageElectric)
  (Variables|Default|SetDamageCorrosive DamageCorrosive)
  (Variables|Default|SetDamageIceWater DamageIceWater)
  (Variables|Default|SetDamageExplosive DamageExplosive))