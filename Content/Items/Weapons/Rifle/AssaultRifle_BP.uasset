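; Assault rifle weapon Blueprint, a child of a weapon base, that fires automatically while the fire input is active.
; FireWeapon calls the parent, shoots once immediately, then starts a looping timer at the firing rate.
; Each shot spawns the projectile class at the transform from CalculateShootInfo while the firing flag is set.
; StopFiringWeapon calls the parent, clears the flag and invalidates the timer.
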(event Custom|AutomaticFire
  (if (Variables|Default|GetisFiring)
    ;[1 1 1] Basic Fire code
    (bind _shoottolocation (CallFunction|CalculateShootInfo))
    (Game|SpawnActorfromClass (Variables|Default|GetProjectileClass) _shoottolocation "Undefined" 0 0)))

(event EventBeginPlay)

(event Collision|EventActorBeginOverlap
  (params (OtherActor :type Actor%20Object%20Reference)))

(event EventTick
  (params (DeltaSeconds :type Float%20%28single-precision%29)))

(event EventFireWeapon
  (|CallParentFunction)
  (Variables|Default|SetisFiring true)
  (CallFunction|AutomaticFire)
  (bind _returnvalue (Utilities|Time|SetTimerbyEvent (delegate Custom|AutomaticFire) (Variables|Default|GetFiringRate) true))
  (Variables|Default|SetTimer _returnvalue))

(event EventStopFiringWeapon
  (|CallParentFunction)
  (Variables|Default|SetisFiring false)
  (Utilities|Time|ClearandInvalidateTimerbyHandle (Variables|Default|GetTimer)))

(fn ConstructionScript
  (|CallParentFunction))