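; Base enemy character Blueprint that tracks health and is destroyed on death.
; HP starts at MaxHP, and the TakeDamage event feeds CalculateHealth, then destroys the actor once IsDead is set.
; CalculateHealth rolls rounded random damage, doubles it for criticals and bone-name-based headshots, then adds unmultiplied elemental damage.
; Explosive damage is summed there but TakeDamage never supplies it, and debug prints report hits and HP.
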(event EventBeginPlay
  (Variables|Default|SetHP (Variables|Default|GetMaxHP)))

(event Collision|EventActorBeginOverlap
  (params (OtherActor :type Actor%20Object%20Reference)))

(event EventTick
  (params (DeltaSeconds :type Float%20%28single-precision%29)))

(event EventTakeDamage
  (params (DamageMin :type Float%20%28single-precision%29) (DamageMax :type Float%20%28single-precision%29) (CritChance :type Float%20%28single-precision%29) (FireDamage :type Float%20%28single-precision%29) (ElectricDamage :type Float%20%28single-precision%29) (CorrosiveDamage :type Float%20%28single-precision%29) (IceWaterDamage :type Float%20%28single-precision%29) (ExplosiveDamage :type Float%20%28single-precision%29) (HitBoneName :type Name) (DamageInstigator :type Actor%20Object%20Reference))
  (CallFunction|CalculateHealth DamageMin DamageMax CritChance FireDamage ElectricDamage CorrosiveDamage IceWaterDamage 0.0 HitBoneName)
  (if (Variables|Default|GetisDead)
    (Actor|DestroyActor)))

(fn ConstructionScript)

(fn CalculateHealth
  (params (DamageMin :type Float%20%28single-precision%29) (Damagemax :type Float%20%28single-precision%29) (DamageCritChance :type Float%20%28single-precision%29) (DamageFire :type Float%20%28single-precision%29) (DamageElectric :type Float%20%28single-precision%29) (DamageCorrosive :type Float%20%28single-precision%29) (DamageIceWater :type Float%20%28single-precision%29) (DamageExplosive :type Float%20%28single-precision%29) (BoneName :type Name))
  (if (not (Variables|Default|GetisDead))
    (LocalVariables|SetLocalElementalDamage (+ DamageFire DamageElectric DamageCorrosive DamageIceWater DamageExplosive))
    (LocalVariables|SetLocalDamage (Math|Conversions|ToFloat(Integer) (Math|Float|Round (Math|Random|RandomFloatinRange DamageMin Damagemax))))
    (Utilities|FlowControl|Sequence
      (:then_0
        (if (<= (Math|Random|RandomFloatinRange 0.0 1e+02) DamageCritChance)
          (LocalVariables|SetLocalDamage (* (LocalVariables|GetLocalDamage) 2.0))
          (Development|PrintString "Critical")))
      (:then_1
        (switch name BoneName
          (:head
            (LocalVariables|SetLocalDamage (* (LocalVariables|GetLocalDamage) 2.0))
            (Development|PrintString "Headshot"))))
      (:then_2
        (bind _output_get (Variables|Default|SetHP (- (Variables|Default|GetHP) (+ (LocalVariables|GetLocalDamage) (LocalVariables|GetLocalElementalDamage)))))
        (Development|PrintString (Utilities|String|ToString(Float) _output_get))
        (if (<= _output_get 0.0)
          (Variables|Default|SetHP 0.0)
          (Variables|Default|SetisDead true))))))