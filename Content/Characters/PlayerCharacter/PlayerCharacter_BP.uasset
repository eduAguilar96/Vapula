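; Player character Blueprint that spawns and carries a weapon, controls its firing and adds air control.
; On BeginPlay it spawns the configured weapon class, attaches it to the mesh's weapon socket and hands it the camera.
; Fire events forward to the equipped weapon, gated by a CanFire flag whose setter stops firing when cleared.
; Movement axes apply camera-yaw-relative input only while falling, with a leftover debug print on forward input.
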(event Custom|FireWeapon
  ;[1 1 1] Fire Weapon
  (if (Variables|Default|GetcanFire)
    (Default|FireWeapon (Variables|Default|GetEquipedWeapon))))

(event Custom|StopFiringEvent
  ;[1 1 1] Fire Weapon
  (Default|StopFiringWeapon (Variables|Default|GetEquipedWeapon)))

(event EventBeginPlay
  (bind _returnvalue (Game|SpawnActorfromClass (Variables|Default|GetWeaponToSpawn) (Transformation|GetActorTransform) "AlwaysSpawn" 0 self))
  (bind _asbase_weapon_bp (Utilities|Casting|CastToBaseWeapon_BP _returnvalue))
  (bind _output_get (Variables|Default|SetEquipedWeapon _asbase_weapon_bp))
  (Class|Actor|AttachRootComponentto _output_get (Variables|Character|GetMesh) "WeaponSocket" "SnapToTarget" true)
  (Default|SetCamera _asbase_weapon_bp (Variables|Default|GetCamera)))

(event Collision|EventActorBeginOverlap
  (params (OtherActor :type Actor%20Object%20Reference)))

(event EventTick
  (params (DeltaSeconds :type Float%20%28single-precision%29)))

(event EventTakeDamage
  (params (DamageMin :type Float%20%28single-precision%29) (DamageMax :type Float%20%28single-precision%29) (CritChance :type Float%20%28single-precision%29) (FireDamage :type Float%20%28single-precision%29) (ElectricDamage :type Float%20%28single-precision%29) (CorrosiveDamage :type Float%20%28single-precision%29) (IceWaterDamage :type Float%20%28single-precision%29) (ExplosiveDamage :type Float%20%28single-precision%29) (HitBoneName :type Name :default "None") (DamageInstigator :type Actor%20Object%20Reference)))

(event Input|AxisEvents|InputAxisMoveForward
  (params (AxisValue :type Float%20%28single-precision%29))
  ;[1 1 1] Air Control (Must disable/overwrite root motion, dont know how)
  (if (AI|Components|NavMovement|IsFalling (Variables|Character|GetCharacterMovement))
    (Pawn|Input|AddMovementInput (Math|Vector|GetForwardVector (Math|Rotator|MakeRotator 0.0 0.0 (.Yaw (Math|Rotator|BreakRotator (Pawn|GetControlRotation :!class /Script/Engine.Pawn))))) AxisValue false)
    (Development|PrintString "Hello")))

(event Input|AxisEvents|InputAxisMoveRight
  (params (AxisValue :type Float%20%28single-precision%29))
  ;[1 1 1] Air Control (Must disable/overwrite root motion, dont know how)
  (if (AI|Components|NavMovement|IsFalling (Variables|Character|GetCharacterMovement))
    (Pawn|Input|AddMovementInput (Math|Vector|GetRightVector (Math|Rotator|MakeRotator 0.0 0.0 (.Yaw (Math|Rotator|BreakRotator (Pawn|GetControlRotation :!class /Script/Engine.Pawn))))) AxisValue false)))

(fn ConstructionScript)

(fn SetCanFire
  (params (canFire :type Boolean))
  (bind _output_get (Variables|Default|SetcanFire canFire))
  (if (not _output_get)
    (CallFunction|StopFiringEvent)))