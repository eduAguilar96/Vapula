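; Player controller for the player character, turning input into state and actions on the cached character Blueprint.
; Movement axes are stored in variables, while look axes apply sensitivity-scaled yaw and pitch with optional Y inversion.
; Sprint and crouch are mutually exclusive toggles, and sprinting, which requires forward input to toggle, updates whether the character can fire.
; Fire input starts and stops the weapon, and jumping adds movement input along the current horizontal velocity.
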(event EventBeginPlay
  (bind _asplayer_character_bp (Utilities|Casting|CastToPlayerCharacter_BP (Game|GetPlayerCharacter 0)))
  (Variables|Default|SetPlayerCharacter _asplayer_character_bp))

(event EventTick
  (params (DeltaSeconds :type Float%20%28single-precision%29)))

(event Input|ActionEvents|InputActionSprint
  (params (Key :type Key%20Structure :default "AnyKey"))
  ;[1 1 1] Sprint Button
  (:Pressed
    (if (> (Variables|Default|GetMoveForward) 0.0)
      (bind _output_get (Variables|Default|SetisSprinting (not (Variables|Default|GetisSprinting))))
      (Variables|Default|SetisCrouching false)
      (Default|SetCanFire (Variables|Default|GetPlayerCharacter) (not _output_get)))))

(event Input|ActionEvents|InputActionCrouch
  (params (Key :type Key%20Structure :default "AnyKey"))
  ;[1 1 1] Crouch Button
  (:Pressed
    (Variables|Default|SetisCrouching (not (Variables|Default|GetisCrouching)))
    (Variables|Default|SetisSprinting false)))

(event Input|ActionEvents|InputActionPrimaryFire
  (params (Key :type Key%20Structure :default "AnyKey"))
  (bind _playercharacter (Variables|Default|GetPlayerCharacter))
  ;[1 1 1] Fire Button
  (:Pressed
    (Default|FireWeapon _playercharacter))
  (:Released
    (Default|StopFiringEvent _playercharacter)))

(event Input|ActionEvents|InputActionJump
  (params (Key :type Key%20Structure :default "AnyKey"))
  (bind _playercharacter (Variables|Default|GetPlayerCharacter))
  (bind _playercharacter_2 (Variables|Default|GetPlayerCharacter))
  (bind _returnvalue (Transformation|GetVelocity _playercharacter_2))
  (bind (_x _y) (Math|Vector|BreakVector _returnvalue))
  ;[1 1 1] Jump Button
  (:Pressed
    (Variables|Default|SetJump true)
    (bind _output_get (Variables|Default|SetairVelocity (Math|Vector|MakeVector _x _y 0.0)))
    (Character|Jump _playercharacter)
    (Pawn|Input|AddMovementInput _playercharacter _output_get (+ _x _y) false))
  (:Released
    (Variables|Default|SetJump false)
    (Character|StopJumping _playercharacter)))

(event Input|AxisEvents|InputAxisMoveForward
  (params (AxisValue :type Float%20%28single-precision%29))
  ;[1 1 1] Get Move Input
  (Variables|Default|SetMoveForward AxisValue))

(event Input|AxisEvents|InputAxisMoveRight
  (params (AxisValue :type Float%20%28single-precision%29))
  ;[1 1 1] Get Move Input
  (Variables|Default|SetMoveRight AxisValue))

(event Input|AxisEvents|InputAxisLookUp
  (params (AxisValue :type Float%20%28single-precision%29))
  (bind _sensitivity (Variables|Default|GetSensitivity))
  (bind _returnvalue (* AxisValue _sensitivity))
  ;[1 1 1] Get Look Input
  (if (Variables|Default|GetInvertY)
    (Class|PlayerController|AddPitchInput (* _returnvalue -1.0))
    (else
      (Class|PlayerController|AddPitchInput _returnvalue))))

(event Input|AxisEvents|InputAxisLookRight
  (params (AxisValue :type Float%20%28single-precision%29))
  ;[1 1 1] Get Look Input
  (Class|PlayerController|AddYawInput (* AxisValue (Variables|Default|GetSensitivity))))

(fn ConstructionScript)

(fn SetSprinting
  (params (IsSprinting :type Boolean))
  (Variables|Default|SetisSprinting IsSprinting))